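; BP_MissionManager runs a linear sequence of missions from a Quests array.
; Shortly after BeginPlay it starts the current quest's mission message, passing itself, and each MissionCompleted call advances the index to the next one.
; After the last quest it calls Hide, which removes all widgets after a delay, while Show creates and displays the BP_MissionUI instruction widget.
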(event EventBeginPlay
  (Utilities|FlowControl|Delay 1.0)
  (Class|BPSingleMission|StartMission(Message) (Utilities|Array|Get(acopy) (Variables|Default|Getquests) (Variables|Default|GetcurrentQuest)) self))

(event EventMissionCompleted
  (bind _quests (Variables|Default|Getquests))
  ;[0.15 0.15 0.15 0.5] Mission Complete - Jerry
  (bind _output_get (Variables|Default|SetcurrentQuest (+ (Variables|Default|GetcurrentQuest) 1)))
  (if (Utilities|Array|IsValidIndex _quests _output_get)
    (Class|BPSingleMission|StartMission(Message) (Utilities|Array|Get(acopy) _quests _output_get) self)
    (else
      (Default|Hide self))))

(event EventHide
  ;[0.15 0.15 0.15 0.5] HIDE UI - Jerry
  (Utilities|FlowControl|Delay (Variables|Default|GethideWidgetTime))
  (Viewport|RemoveAllWidgets))

(event EventShow
  ;[0.15 0.15 0.15 0.5] SHOW UI - Jerry
  (bind _returnvalue (UserInterface|CreateWidget "/Game/Scripts/UI/BP_MissionUI.BP_MissionUI_C" (Game|GetPlayerController 0)))
  (bind _output_get (Variables|Default|SetinstructionWidget _returnvalue))
  (UserInterface|Viewport|AddtoViewport _output_get 0))

(fn ConstructionScript)