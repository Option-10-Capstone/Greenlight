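; Spline actor that lays copies of a static mesh along its spline in the construction script, with collision enabled.
; Mesh bounds on the forward axis set segment length.
; Spaced mode places rotated, undeformed pieces at spacing intervals; otherwise segments bend end to end, with tangents clamped to mesh length.
; Bent segments take their up direction from interpolated per-point UpVectors entries, with optional debug arrows at spline points.
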(event EventBeginPlay)

(event Collision|EventActorBeginOverlap
  (params (OtherActor :type Actor%20Object%20Reference)))

(event EventTick
  (params (DeltaSeconds :type Float%20%28single-precision%29)))

(fn ConstructionScript
  (bind _splinemesh (Variables|Default|GetsplineMesh))
  (bind _spline (Variables|Default|GetSpline))
  (bind _spline_2 (Variables|Default|GetSpline))
  (bind _spline_3 (Variables|Default|GetSpline))
  (bind _returnvalue (StaticMesh|GetBoundingBox _splinemesh))
  (bind _returnvalue_2 (Spline|GetSplineLength _spline_2))
  (bind _returnvalue_3 (- (.max _returnvalue) (.min _returnvalue)))
  (if (Utilities|Enum|Equal(Enum) (Variables|Default|GetinForwardAxis) "X")
    (Variables|Default|SetmeshLength (.x _returnvalue_3))
    (elif (Utilities|Enum|Equal(Enum) (Variables|Default|GetinForwardAxis) "Y")
      (Variables|Default|SetmeshLength (.y _returnvalue_3))
      (else
        (Variables|Default|SetmeshLength (.z _returnvalue_3)))))
  (if (Variables|Debug|GetdoSpaceMeshes)
    (Variables|Default|SetsectionLength (+ (Variables|Default|Getspacing) (Variables|Default|GetmeshLength)))
    (for _index (range 0 (Math|Float|Truncate (/ (Spline|GetSplineLength (Variables|Default|GetSpline)) (Variables|Default|GetsectionLength))))
      (Variables|Default|Setindex _index)
      (bind _returnvalue_4 (AddComponent|AddSplineMeshComponent false (Math|Transform|MakeTransform (Spline|GetLocationatDistanceAlongSpline _spline (* (Variables|Default|Getindex) (Variables|Default|GetsectionLength)) "Local") (Math|Rotator|CombineRotators (Variables|Default|GetmeshRotation) (Spline|GetRotationatDistanceAlongSpline _spline (* (Variables|Default|Getindex) (Variables|Default|GetsectionLength)) "Local")))))
      (Components|StaticMesh|SetStaticMesh _returnvalue_4 (Variables|Default|GetsplineMesh))
      (Collision|SetCollisionEnabled _returnvalue_4 "QueryAndPhysics")
      (SplineMesh|SetForwardAxis _returnvalue_4 "X" true))
    (else
      (for _index_2 (range 0 (Math|Float|Truncate (/ (Spline|GetSplineLength (Variables|Default|GetSpline)) (Variables|Default|GetmeshLength))))
        (Variables|Default|Setindex _index_2)
        (bind _returnvalue_5 (AddComponent|AddSplineMeshComponent false))
        (Components|StaticMesh|SetStaticMesh _returnvalue_5 (Variables|Default|GetsplineMesh))
        (Collision|SetCollisionEnabled _returnvalue_5 "QueryAndPhysics")
        (SplineMesh|SetForwardAxis _returnvalue_5 (Variables|Default|GetinForwardAxis) true)
        (bind (_location _tangent) (CallFunction|GetLocationandTangent (Variables|Default|Getindex)))
        (bind (_location_2 _tangent_2) (CallFunction|GetLocationandTangent (+ (Variables|Default|Getindex) 1)))
        (SplineMesh|SetStartandEnd _returnvalue_5 _location _tangent _location_2 _tangent_2 true :!class /Script/Engine.SplineMeshComponent)
        (Variables|Default|SetinputKey (Class|SplineComponent|GetInputKeyValueatDistanceAlongSpline (Variables|Default|GetSpline) (/ (+ (* (Variables|Default|Getindex) (Variables|Default|GetmeshLength)) (Math|Float|SelectFloat (+ (* (Variables|Default|Getindex) (Variables|Default|GetmeshLength)) (Variables|Default|GetmeshLength)) _returnvalue_2 (< (+ (* (Variables|Default|Getindex) (Variables|Default|GetmeshLength)) (Variables|Default|GetmeshLength)) _returnvalue_2))) 2.0)))
        (if true
          (SplineMesh|SetSplineUpDir _returnvalue_5 (Math|Vector|Lerp(Vector) (.Value (Utilities|Map|Find (Variables|Default|GetupVectors) (Math|Float|Ceil (Variables|Default|GetinputKey)))) (.Value (Utilities|Map|Find (Variables|Default|GetupVectors) (Math|Float|Floor (Variables|Default|GetinputKey)))) (Math|Float|Fraction (Variables|Default|GetinputKey))) true)
          (else
            (SplineMesh|SetSplineUpDir _returnvalue_5 (Class|SplineComponent|GetUpVectoratDistanceAlongSpline (Variables|Default|GetSpline) (+ (/ (- (Math|Float|SelectFloat (+ (* (Variables|Default|Getindex) (Variables|Default|GetmeshLength)) (Variables|Default|GetmeshLength)) _returnvalue_2 (< (+ (* (Variables|Default|Getindex) (Variables|Default|GetmeshLength)) (Variables|Default|GetmeshLength)) _returnvalue_2)) (* (Variables|Default|Getindex) (Variables|Default|GetmeshLength))) 2.0) (Math|Float|SelectFloat (+ (* (Variables|Default|Getindex) (Variables|Default|GetmeshLength)) (Variables|Default|GetmeshLength)) _returnvalue_2 (< (+ (* (Variables|Default|Getindex) (Variables|Default|GetmeshLength)) (Variables|Default|GetmeshLength)) _returnvalue_2))) "Local") true)))
        (if (Variables|Debug|GetshowUpVector)
          (AddComponent|AddArrowComponent false (Math|Transform|MakeTransform (Spline|GetLocationatSplinePoint _spline_3 (Variables|Default|Getindex) "Local") (Math|Rotator|CombineRotators "90.000000,0.000000,0.000000" (Spline|GetRotationatSplinePoint _spline_3 (Variables|Default|Getindex) "Local")) "3.000000,3.000000,3.000000")))))))

(fn GetLocationandTangent
  (params (A :type Integer))
  (bind _spline (Variables|Default|GetSpline))
  (bind _meshlength (Variables|Default|GetmeshLength))
  (bind _returnvalue (* A _meshlength))
  (return (Spline|GetLocationatDistanceAlongSpline _spline _returnvalue "Local") (Math|Vector|ClampVectorSize (Spline|GetTangentatDistanceAlongSpline _spline _returnvalue "Local") 0.0 (Variables|Default|GetmeshLength))))